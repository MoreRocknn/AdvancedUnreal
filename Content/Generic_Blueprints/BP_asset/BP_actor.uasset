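; Interactable hinged door actor that swings open and closed around its DoorPivot on each Interact.
; Interact flips IsOpen, and SetOpen plays or reverses OpenDoorTimeline.
; The timeline update derives pivot yaw linearly from playback progress times OpenAngle, with length set by AnimationDuration.
; BeginPlay moves the timeline to its end in both IsOpen branches, including the closed one.
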(event `self.ReceiveBeginPlay`
  (bind _opendoortimeline (`self.OpenDoorTimeline`))
  (bind _returnvalue (`TimelineComponent.GetTimelineLength` _opendoortimeline))
  (`TimelineComponent.SetTimelineLength` (`self.OpenDoorTimeline`) (`self.AnimationDuration`))
  (if (`self.IsOpen`)
    (`TimelineComponent.SetNewTime` _opendoortimeline _returnvalue)
    (else
      (`TimelineComponent.SetNewTime` _opendoortimeline _returnvalue))))

(event `/Game/FirstPerson/Blueprints/BP_GenericBP.Interact`
  (bind _output_get (set `self.IsOpen` (not (`self.IsOpen`))))
  (`self.SetOpen` _output_get))

(fn `SetOpen`
  (params (Open :type Boolean))
  (bind _opendoortimeline (`self.OpenDoorTimeline`))
  (if Open
    (`TimelineComponent.Play` _opendoortimeline)
    (else
      (`TimelineComponent.Reverse` _opendoortimeline))))

(fn `UserConstructionScript`)